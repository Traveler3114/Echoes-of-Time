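; Default game mode that handles level changes and pausing for a listen-server multiplayer game.
; NextLevel server-travels to the named level with listen and game mode URL options, then calls LoadingScreen on every BP_GameController.
; PauseGame records the requesting controller and pauses the game, and UnpauseGame resumes it only when called with that same controller.
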(event `NextLevel`
  (params (LevelName :type String))
  (`AdvancedSessionsLibrary.ServerTravel` (`KismetStringLibrary.Concat_StrStr` LevelName "?listen?game=/Game/Blueprints/GameMode/DefaultGameMode"))
  (bind _outactors (`GameplayStatics.GetAllActorsOfClass` "/Game/Blueprints/Controller/BP_GameController.BP_GameController_C"))
  (for _array_element _outactors
    (`/Game/Blueprints/Controller/BP_GameController.LoadingScreen` _array_element)))

(event `PauseGame`
  (params (PC :type "PlayerController Object Reference"))
  (set `self.PausingPC` PC)
  (`GameplayStatics.SetGamePaused` true))

(event `UnpauseGame`
  (params (PC :type "PlayerController Object Reference"))
  (if (== PC (`self.PausingPC`))
    (`GameplayStatics.SetGamePaused` false)))

(fn `UserConstructionScript`)