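; Lobby player controller that manages a player's lobby UI, info and ready status.
; On BeginPlay, the local controller shows the cursor, creates the lobby widget and calls SetPlayerNameOnServer.
; That event and the R-key ready toggle update the player info struct and pass the controller to BP_LobbyGameMode, with a delayed retry event available.
; OnStartMatch shows a loading widget and disables input.
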(event `self.ReceiveBeginPlay`
  (`self.SetUp`))

(event `TryAgainUpdatingLobbyInfo`
  (`KismetSystemLibrary.Delay` 0.2)
  (bind _asbp_lobby_game_mode (cast `/Game/Blueprints/GameMode/BP_LobbyGameMode` (`GameplayStatics.GetGameMode`)))
  (`/Game/Blueprints/GameMode/BP_LobbyGameMode.UpdatePlayerLobbyInfo` _asbp_lobby_game_mode self))

(event `SetPlayerNameOnServer`
  (setmembers `/Game/Blueprints/S_PlayerLobbyInfo` :`StructRef` (`self.PlayerLobbyInfoPC`))
  (bind _asbp_lobby_game_mode (cast `/Game/Blueprints/GameMode/BP_LobbyGameMode` (`GameplayStatics.GetGameMode`)))
  (`/Game/Blueprints/GameMode/BP_LobbyGameMode.UpdatePlayerLobbyInfo` _asbp_lobby_game_mode self))

(event `ToggleReadyStatusOnServer`
  (bind _playerlobbyinfopc (`self.PlayerLobbyInfoPC`))
  (setmembers `/Game/Blueprints/S_PlayerLobbyInfo` :`StructRef` _playerlobbyinfopc :`IsReady` (not (`.IsReady_11_37DA0A5F4770D6A394CCFF998C121246` (break `/Game/Blueprints/S_PlayerLobbyInfo` _playerlobbyinfopc))))
  (bind _asbp_lobby_game_mode (cast `/Game/Blueprints/GameMode/BP_LobbyGameMode` (`GameplayStatics.GetGameMode`)))
  (`/Game/Blueprints/GameMode/BP_LobbyGameMode.UpdatePlayerLobbyInfo` _asbp_lobby_game_mode self))

(event `Key|R`
  (params (Key :type "Key Structure"))
  (:`Pressed`
    (`self.ToggleReadyStatusOnServer`)))

(event `OnStartMatch`
  (bind _returnvalue (`|CreateWidget` "/Game/Blueprints/Widgets/WBP_Loading.WBP_Loading_C"))
  (`UserWidget.AddToViewport` _returnvalue 0)
  (`self.DisableInput` self))

(fn `SetUp`
  (if (`self.IsLocalPlayerController`)
    (set `self.bShowMouseCursor` true)
    (`WidgetBlueprintLibrary.SetInputMode_GameAndUIEx` self null "DoNotLock" false)
    (bind _returnvalue (`|CreateWidget` "/Game/Blueprints/Widgets/LobbyWidgets/WBP_LobbyUI.WBP_LobbyUI_C"))
    (bind _output_get (set `self.LobbyUI_Ref` _returnvalue))
    (`UserWidget.AddToViewport` _output_get 0)
    (`self.SetPlayerNameOnServer`)))

(fn `UserConstructionScript`)