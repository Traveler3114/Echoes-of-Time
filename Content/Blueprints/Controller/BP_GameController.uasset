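; BP_GameController is a player controller that handles game input mode, the loading screen and the pause menu.
; LoadingScreen shows the loading widget for the local controller and disables input.
; Escape and Q share one FlipFlop that alternately creates and removes the pause menu.
; Pause and unpause requests go to the game mode through interface messages, passing the controller along.
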(event `self.ReceiveBeginPlay`
  (set `self.bShowMouseCursor` false)
  (`WidgetBlueprintLibrary.SetInputMode_GameOnly` self))

(event `LoadingScreen`
  (if (`self.IsLocalPlayerController` self)
    (bind _returnvalue (`|CreateWidget` "/Game/Blueprints/Widgets/WBP_Loading.WBP_Loading_C"))
    (`UserWidget.AddToViewport` _returnvalue 0)
    (`self.DisableInput` self)))

(event `Key|Escape`
  (params (Key :type "Key Structure"))
  ; Pausing
  (:`Pressed`
    (`/Engine/EditorBlueprintResources/StandardMacros.FlipFlop` :!label _label
      (:`A`
        (bind _returnvalue (`|CreateWidget` "/Game/Blueprints/Widgets/WBP_PauseMenu.WBP_PauseMenu_C"))
        (bind _output_get (set `self.PauseMenuRef` _returnvalue))
        (`UserWidget.AddToViewport` _output_get 0)
        (if (not (`GameplayStatics.IsGamePaused`))
          (`self.PCPauseGame`)))
      (:`B`
        (`Widget.RemoveFromParent` (`self.PauseMenuRef`))
        (set `self.PauseMenuRef` null)
        (`self.PCUnpauseGame`)
        (set `self.bShowMouseCursor` false)))))

(event `Key|Q` :paused true
  (params (Key :type "Key Structure"))
  ; Pausing
  (:`Pressed`
    (goto _label)))

(event `PCPauseGame`
  ; Pausing
  (message `/Game/Blueprints/Interfaces/BPI_DefaultGameMode.PauseGameInterface` (`GameplayStatics.GetGameMode`) self))

(event `PCUnpauseGame`
  ; Pausing
  (message `/Game/Blueprints/Interfaces/BPI_DefaultGameMode.UnpauseGameInterface` (`GameplayStatics.GetGameMode`) self))

(fn `UserConstructionScript`)