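; Game instance for a two-player game that manages online sessions and saved games, with create, save and load exposed through interface events.
; It hosts a Lobby listen server and joins accepted invites after destroying the current session.
; Saves store level path and both players' transforms in incrementally numbered slots, indexed by a MetaSave object.
; Loading sets ShouldLoad and either passes the map to the main-menu GameMode or server-travels behind loading screens.
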(event `CreateServer`
  (`CreateSessionCallbackProxyAdvanced.CreateAdvancedSession` :`PlayerController` (`GameplayStatics.GetPlayerController` 0) :`PublicConnections` 2
    (:`OnSuccess`
      (`GameplayStatics.OpenLevelBySoftObjectPtr` "/Game/Maps/Lobby.Lobby" true "listen"))))

(event `self.OnSessionInviteAccepted`
  (params (LocalPlayerNum :type Integer) (PersonInvited :type "BPUniqueNetId Structure") (SessionToJoin :type "BlueprintSessionResult Structure (by ref)"))
  (`DestroySessionCallbackProxy.DestroySession` (`GameplayStatics.GetPlayerController` 0)
    (:`OnSuccess`
      _)
    (:`OnFailure`
      _))
  (`JoinSessionCallbackProxy.JoinSession` null SessionToJoin))

(event `Save`
  (bind _saves (`/Game/Blueprints/SaveLoad/BP_MetaSave.Saves` (`self.MetaSave`)))
  (bind _returnvalue (`KismetStringLibrary.Concat_StrStr` "Save" " " (`KismetStringLibrary.Conv_IntToString` (+ (`KismetStringLibrary.Conv_StringToInt` (`.RightS` (`KismetStringLibrary.Split` (`|GetArrayItem` _saves (`KismetArrayLibrary.Array_LastIndex` _saves)) " "))) 1))))
  (bind _returnvalue_2 (`GameplayStatics.LoadGameFromSlot` "MetaSave"))
  (if (== null _returnvalue_2)
    (bind _returnvalue_3 (`GameplayStatics.CreateSaveGameObject` "/Game/Blueprints/SaveLoad/BP_MetaSave.BP_MetaSave_C"))
    (set `self.MetaSave` _returnvalue_3)
    (else
      (bind _asbp_meta_save (cast `/Game/Blueprints/SaveLoad/BP_MetaSave` _returnvalue_2))
      (set `self.MetaSave` _asbp_meta_save)))
  (bind _returnvalue_4 (`self.GetLevelPath`))
  (bind _structout (setmembers `/Game/Blueprints/SaveLoad/S_SaveInfo` :`StructRef` (`self.SaveInfo`) :`Map` _returnvalue_4 :`Player1Trasnform` (`Actor.GetTransform` (`GameplayStatics.GetPlayerPawn` 0)) :`Player2Trasnform` (`Actor.GetTransform` (`GameplayStatics.GetPlayerPawn` 1))))
  (bind _returnvalue_5 (`GameplayStatics.CreateSaveGameObject` "/Game/Blueprints/SaveLoad/BP_SaveObject.BP_SaveObject_C"))
  (set `/Game/Blueprints/SaveLoad/BP_SaveObject.SaveInfo` _structout _returnvalue_5)
  (`GameplayStatics.SaveGameToSlot` _returnvalue_5 _returnvalue)
  (`KismetArrayLibrary.Array_Add` (`/Game/Blueprints/SaveLoad/BP_MetaSave.Saves` (`self.MetaSave`)) _returnvalue)
  (`GameplayStatics.SaveGameToSlot` (`self.MetaSave`) "MetaSave"))

(event `Load`
  (params (Save :type String))
  (bind _saveinfo_map (break `/Game/Blueprints/SaveLoad/S_SaveInfo` (`self.SaveInfo`)))
  (bind _saveinfo_map_2 (break `/Game/Blueprints/SaveLoad/S_SaveInfo` (`self.SaveInfo`)))
  (bind _returnvalue (`GameplayStatics.LoadGameFromSlot` Save))
  (bind _asbp_save_object (cast `/Game/Blueprints/SaveLoad/BP_SaveObject` _returnvalue))
  (set `self.SaveInfo` (`/Game/Blueprints/SaveLoad/BP_SaveObject.SaveInfo` _asbp_save_object))
  (bind _returnvalue_2 (`GameplayStatics.GetCurrentLevelName` true))
  (if (`KismetStringLibrary.EqualEqual_StrStr` _returnvalue_2 "MainMenuMap")
    (message `/Game/Blueprints/Interfaces/BPI_LobbyGameMode.SetSavedLevelInterface` (`GameplayStatics.GetGameMode`) _saveinfo_map)
    (set `self.bShouldLoad` true)
    (else
      (`AdvancedSessionsLibrary.ServerTravel` (`KismetStringLibrary.Concat_StrStr` _saveinfo_map_2 "?listen?game=/Game/Blueprints/GameMode/DefaultGameMode"))
      (message `/Game/Blueprints/Interfaces/BPI_GameController.LoadingScreenInterface` (`GameplayStatics.GetPlayerController` 0))
      (message `/Game/Blueprints/Interfaces/BPI_GameController.LoadingScreenInterface` (`GameplayStatics.GetPlayerController` 1))
      (set `self.bShouldLoad` true))))

(event `/Game/Blueprints/Interfaces/BPI_MyGameInstance.CreateServerInterface`
  ; Interfaces
  (`self.CreateServer`))

(event `/Game/Blueprints/Interfaces/BPI_MyGameInstance.SaveInterface`
  ; Interfaces
  (`self.Save`))

(event `/Game/Blueprints/Interfaces/BPI_MyGameInstance.LoadInterface`
  (params (Save :type String))
  ; Interfaces
  (`self.Load` Save))