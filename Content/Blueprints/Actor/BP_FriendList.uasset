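; BP_FriendList is a world-space friend list actor that a lobby player platform shows or hides.
; Show toggles visibility, tells the previously recorded platform to turn off its friend list, then stores the new platform or clears it.
; Each tick while visible, it projects the mouse ray out to the actor's distance and hides itself when that point strays too far from its location.
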(event `self.ReceiveTick`
  (params (DeltaSeconds :type "Float (single-precision)"))
  (`self.CheckToHideFriendList`))

(fn `CheckToHideFriendList`
  (bind (_worldlocation _worlddirection) (`PlayerController.DeprojectMousePositionToWorld` (`GameplayStatics.GetPlayerController` 0)))
  (if (`self.bHidden`)
    _
    (elif (not (== (+ _worldlocation (* (`KismetMathLibrary.Vector_Distance` (`self.K2_GetActorLocation`) _worldlocation) _worlddirection)) (`self.K2_GetActorLocation`) :`ErrorTolerance` 200.0))
      (`self.Show` false))))

(fn `Show`
  (params (bShow :type Boolean) (FromLobbyPlayerPlatform :type "/Game/Blueprints/Actor/BP_LobbyPlayerPlatform Object Reference"))
  (if bShow
    (`self.SetActorHiddenInGame` false)
    (bind _lastlobbyplayer (`self.LastLobbyPlayer`)
      (:`then`
        (`/Game/Blueprints/Actor/BP_LobbyPlayerPlatform.ShowFriendList` _lastlobbyplayer false))
      (:`else`
        _))
    (set `self.LastLobbyPlayer` (`local.FromLobbyPlayerPlatform`))
    (else
      (`self.SetActorHiddenInGame` true)
      (bind _lastlobbyplayer_2 (`self.LastLobbyPlayer`)
        (:`then`
          (`/Game/Blueprints/Actor/BP_LobbyPlayerPlatform.ShowFriendList` _lastlobbyplayer_2 false))
        (:`else`
          _))
      (set `self.LastLobbyPlayer` null))))

(fn `UserConstructionScript`)